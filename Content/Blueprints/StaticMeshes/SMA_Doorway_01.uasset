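; Doorway static mesh actor that can fade its outside and inside surfaces to partial transparency and back.
; The construction script creates dynamic instances of the outside and inside materials and assigns them to the mesh's two material slots.
; FadeStart plays a timeline that drives both Opacity parameters from opaque toward the given Scale as the fade curve rises.
; FadeEnd reverses the same timeline to undo the fade.
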(event `/Game/Blueprints/Interfaces/I_FadeObject.Fade Start`
  (params (Scale :type "Float (double-precision)"))
  (bind (_direction _fade) (`Timeline|Timeline` :!label _label)
    (:`Update`
      (bind _returnvalue (- 1.0 (* _fade (- 1.0 Scale))))
      (`MaterialInstanceDynamic.SetScalarParameterValue` (`self.Dynamic Material Outside`) "Opacity" _returnvalue)
      (`MaterialInstanceDynamic.SetScalarParameterValue` (`self.Dynamic Material Inside`) "Opacity" _returnvalue))))

(event `/Game/Blueprints/Interfaces/I_FadeObject.Fade End`
  (goto _label :!via `Reverse`))

(fn `UserConstructionScript`
  (bind _staticmeshcomponent (`self.StaticMeshComponent`))
  (bind _returnvalue (`KismetMaterialLibrary.CreateDynamicMaterialInstance` (`self.Material Outside`)))
  (bind _output_get (set `self.Dynamic Material Outside` _returnvalue))
  (`PrimitiveComponent.SetMaterial` _staticmeshcomponent 0 _output_get)
  (bind _returnvalue_2 (`KismetMaterialLibrary.CreateDynamicMaterialInstance` (`self.Material Inside`)))
  (bind _output_get_2 (set `self.Dynamic Material Inside` _returnvalue_2))
  (`PrimitiveComponent.SetMaterial` _staticmeshcomponent 1 _output_get_2))